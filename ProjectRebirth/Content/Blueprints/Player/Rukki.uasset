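; Rukki is a player character Blueprint that sets up limb hit volumes for melee attacks.
; The construction script attaches the hand and leg components to hand and shin bone sockets on the mesh, so they follow the animation.
; Each component's begin-overlap event forwards its full hit data to a shared OnHitWithAttack handler, which is defined outside these graphs.
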(event OnComponentBeginOverlap(RightLeg)
  (params (OverlappedComponent :type Primitive%20Component%20Object%20Reference) (OtherActor :type Actor%20Object%20Reference) (OtherComp :type Primitive%20Component%20Object%20Reference) (OtherBodyIndex :type Integer) (bFromSweep :type Boolean) (SweepResult :type Hit%20Result%20Structure%20%28by%20ref%29))
  (Class|Rukki|OnHitwithAttack OverlappedComponent OtherActor OtherComp OtherBodyIndex bFromSweep SweepResult))

(event OnComponentBeginOverlap(LeftHand)
  (params (OverlappedComponent :type Primitive%20Component%20Object%20Reference) (OtherActor :type Actor%20Object%20Reference) (OtherComp :type Primitive%20Component%20Object%20Reference) (OtherBodyIndex :type Integer) (bFromSweep :type Boolean) (SweepResult :type Hit%20Result%20Structure%20%28by%20ref%29))
  (Class|Rukki|OnHitwithAttack OverlappedComponent OtherActor OtherComp OtherBodyIndex bFromSweep SweepResult))

(event OnComponentBeginOverlap(RightHand)
  (params (OverlappedComponent :type Primitive%20Component%20Object%20Reference) (OtherActor :type Actor%20Object%20Reference) (OtherComp :type Primitive%20Component%20Object%20Reference) (OtherBodyIndex :type Integer) (bFromSweep :type Boolean) (SweepResult :type Hit%20Result%20Structure%20%28by%20ref%29))
  (Class|Rukki|OnHitwithAttack OverlappedComponent OtherActor OtherComp OtherBodyIndex bFromSweep SweepResult))

(event OnComponentBeginOverlap(LeftLeg)
  (params (OverlappedComponent :type Primitive%20Component%20Object%20Reference) (OtherActor :type Actor%20Object%20Reference) (OtherComp :type Primitive%20Component%20Object%20Reference) (OtherBodyIndex :type Integer) (bFromSweep :type Boolean) (SweepResult :type Hit%20Result%20Structure%20%28by%20ref%29))
  (Class|Rukki|OnHitwithAttack OverlappedComponent OtherActor OtherComp OtherBodyIndex bFromSweep SweepResult))

(event EventBeginPlay)

(event Collision|EventActorBeginOverlap
  (params (OtherActor :type Actor%20Object%20Reference)))

(event EventTick
  (params (DeltaSeconds :type Float%20%28single-precision%29)))

(fn ConstructionScript
  (bind _mesh (Variables|Character|GetMesh))
  (Transformation|AttachComponentToComponent (Variables|Default|GetLeftHand) _mesh "DEF-hand_L" "KeepRelative" "KeepRelative" "KeepWorld" false)
  (Transformation|AttachComponentToComponent (Variables|Default|GetRightHand) _mesh "DEF-hand_R" "KeepRelative" "KeepRelative" "KeepWorld" true)
  (Transformation|AttachComponentToComponent (Variables|Default|GetRightLeg) _mesh "DEF-shin_R_001" "KeepRelative" "KeepRelative" "KeepWorld" false)
  (Transformation|AttachComponentToComponent (Variables|Default|GetLeftLeg) _mesh "DEF-shin_L_001" "KeepRelative" "KeepRelative" "KeepWorld" false))