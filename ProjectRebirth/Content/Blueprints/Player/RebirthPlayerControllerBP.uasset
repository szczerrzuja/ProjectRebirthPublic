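; Player controller Blueprint that keeps the HUD's health and mana displays current and handles player respawning.
; Every tick, it reads the current and max HP and MP from the Rukki character's StatsComponent and pushes them to PlayerHUD, guarded by validity checks.
; A Respawn event asks the ProjectRebirth game mode to restart this player at the SpawnPoint's respawn transform.
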(event EventBeginPlay)

(event EventTick
  (params (DeltaSeconds :type Float%20%28single-precision%29))
  (bind _playerhud (Variables|Default|GetPlayerHUD))
  (bind _rukkiptr (Variables|Default|GetRukkiPtr))
  (bind _statscomponent (Variables|/Script/ProjectRebirth.EntityInterface|GetStatsComponent _rukkiptr))
  (Utilities|IsValid _rukkiptr
    (:Is%20Valid
      (Utilities|IsValid _playerhud
        (:Is%20Valid
          (bind _returnvalue (Class|BaseStatsComponent|GetRegenarative _statscomponent 1))
          (Class|RukkiHUD|SetHPLevel _playerhud (.value (Utilities|Struct|BreakUStatRegen _returnvalue)) (.Max_value (Utilities|Struct|BreakUStatRegen _returnvalue)))
          (bind _returnvalue_2 (Class|BaseStatsComponent|GetRegenarative _statscomponent 2))
          (Class|RukkiHUD|SetMPLevel _playerhud (.value (Utilities|Struct|BreakUStatRegen _returnvalue_2)) (.Max_value (Utilities|Struct|BreakUStatRegen _returnvalue_2))))))))

(event EventRespawn
  (bind _asproject_rebirth_game_mode_base (Utilities|Casting|CastToProjectRebirthGameModeBase (Game|GetGameMode)))
  (bind _returnvalue (Class|PlayerRespawnPoint|GetRespawnTransform (Variables|Default|GetSpawnPoint)))
  (Class|GameModeBase|RestartPlayeratTransform _asproject_rebirth_game_mode_base self _returnvalue))

(fn ConstructionScript)